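; GameplayGM is the networked game mode Blueprint that tracks players, spawns their characters and handles logout.
; Player controllers arriving through SwapPlayerControllers are stored in an array and set to game-only input.
; RespawnPlayer spawns the given character class at a random PlayerStart, adjusting for collisions but always spawning, and possesses it.
; On logout, it calls DestroySessionCaller on GameInfoInstance for the exiting GameplayPC.
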(event `self.K2_OnSwapPlayerControllers`
  (params (OldPC :type "PlayerController Object Reference") (NewPC :type "PlayerController Object Reference"))
  ;[0 0 0] Keeps tracks of Connected Player Controllers
  (`KismetArrayLibrary.Array_Add` (`self.AllPlayerControllers`) NewPC)
  (`WidgetBlueprintLibrary.SetInputMode_GameOnly` NewPC))

(event `RespawnPlayer`
  (params (PlayerController :type "PlayerController Object Reference") (PlayerCharacter :type "Character Class Reference"))
  (bind _spawnpoints (`self.SpawnPoints`))
  ;[0 0 0] Spawn the player with the selected character from the GameplayPC
  (bind _outactors (`GameplayStatics.GetAllActorsOfClass` "/Script/Engine.PlayerStart"))
  (set `self.SpawnPoints` _outactors)
  (bind _returnvalue (`|SpawnActorFromClass` PlayerCharacter (`self.GetTransform` (`|GetArrayItem` _spawnpoints (`KismetMathLibrary.RandomIntegerInRange` 0 (- (`KismetArrayLibrary.Array_Length` _spawnpoints) 1)))) "AdjustIfPossibleButAlwaysSpawn" "OverrideRootScale" null null))
  (`Controller.Possess` PlayerController _returnvalue))

(event `self.K2_OnLogout`
  (params (ExitingController :type "Controller Object Reference"))
  ;[0 0 0] Event OnLogout - Destroy Session Caller
  (bind _asgameplay_pc (cast `/Game/Network/Blueprints/Gameplay/GameplayPC` ExitingController))
  (bind _asgame_info_instance (cast `/Game/Network/Blueprints/AllLevels/GameInfoInstance` (`GameplayStatics.GetGameInstance`)))
  (`/Game/Network/Blueprints/AllLevels/GameInfoInstance.DestroySessionCaller` _asgame_info_instance _asgameplay_pc))

(fn `UserConstructionScript`)