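; BP_GrenadeTest is a test grenade actor launched as a physics object with the throwing character's toss velocity.
; On BeginPlay it casts its instigator to SCharacter and applies the ThrowableComponent's TossVelocity to the mesh as a mass-independent velocity-change impulse.
; The first Hit event sets the mesh's linear damping through a DoOnce, so its motion decays after impact.
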(event `self.ReceiveBeginPlay`
  (bind _asscharacter (cast `SCharacter` (`self.GetInstigator`)))
  (bind _throwparams (`SThrowableComponent.ThrowParams` (`SCharacter.ThrowableComponent` _asscharacter)))
  (`PrimitiveComponent.AddImpulse` (`self.MeshComp`) (`KismetMathLibrary.MakeVector` (break `Vector_NetQuantize` (`.TossVelocity` (break `ThrowParameters` _throwparams))) (`.Y` (break `Vector_NetQuantize` (`.TossVelocity` (break `ThrowParameters` _throwparams)))) (`.Z` (break `Vector_NetQuantize` (`.TossVelocity` (break `ThrowParameters` _throwparams))))) "None" true))

(event `self.ReceiveHit`
  (params (MyComp :type "PrimitiveComponent Object Reference") (Other :type "Actor Object Reference") (OtherComp :type "PrimitiveComponent Object Reference") (bSelfMoved :type Boolean) (HitLocation :type "Vector Structure") (HitNormal :type "Vector Structure") (NormalImpulse :type "Vector Structure") (Hit :type "HitResult Structure (by ref)"))
  (`/Engine/EditorBlueprintResources/StandardMacros.DoOnce` false
    (:`Completed`
      (`PrimitiveComponent.SetLinearDamping` (`self.MeshComp`) 1.5))))

(fn `UserConstructionScript`)